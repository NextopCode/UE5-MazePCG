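; BP_Cell is a maze cell actor with four walls (Left, Front, Right, Back) used by maze generation.
; It records neighboring cells by direction, and RemoveWall hides the chosen wall and disables its collision to open a passage.
; BlowUp runs Convert to Destructible on each wall, swapping any still-visible one for a unit-scale BP_CellDestructible actor spawned at its location and rotation.
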(event `Make Neighbor`
  (params (Direction :type "/Game/MazeGeneration/CellDirection Enum" :default "NewEnumerator0") (`Other Cell` :type "/Game/MazeGeneration/BP_Cell Object Reference"))
  (`BlueprintMapLibrary.Map_Add` (`self.Neighbors`) Direction `Other Cell`))

(event `Remove Wall`
  (params (Direction :type "/Game/MazeGeneration/CellDirection Enum" :default "NewEnumerator0"))
  (bind _left (`self.Left`))
  (bind _right (`self.Right`))
  (bind _front (`self.Front`))
  (bind _back (`self.Back`))
  (switch `/Game/MazeGeneration/CellDirection` Direction
    (:`NewEnumerator0`
      (`SceneComponent.SetVisibility` _left false true)
      (`PrimitiveComponent.SetCollisionEnabled` _left "NoCollision"))
    (:`NewEnumerator1`
      (`SceneComponent.SetVisibility` _front false true)
      (`PrimitiveComponent.SetCollisionEnabled` _front "NoCollision"))
    (:`NewEnumerator2`
      (`SceneComponent.SetVisibility` _right false true)
      (`PrimitiveComponent.SetCollisionEnabled` _right "NoCollision"))
    (:`NewEnumerator3`
      (`SceneComponent.SetVisibility` _back false true)
      (`PrimitiveComponent.SetCollisionEnabled` _back "NoCollision"))))

(event `Blow Up`
  (`self.Convert to Destructible` (`self.Right`))
  (`self.Convert to Destructible` (`self.Left`))
  (`self.Convert to Destructible` (`self.Front`))
  (`self.Convert to Destructible` (`self.Back`)))

(fn `UserConstructionScript`)