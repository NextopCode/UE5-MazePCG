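; Grid actor for maze generation that spawns a SizeX by SizeY field of cell actors and links them as neighbors.
; MakeGrid spawns and destroys a temporary cell to measure its bounds, then places cells at that spacing from the actor's transform into a flat, row-major array.
; A final pass uses GetCell lookups to connect each BP_Cell both ways with its lower-X and lower-Y neighbors, covering every adjacent pair once.
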(fn `Get Cell`
  (params (X :type Integer) (Y :type Integer))
  (returns (Cell :type "Actor Object Reference"))
  (return (`|GetArrayItem` (`self.Cells`) (+ X (* Y (`self.SizeX`))))))

(fn `Make Grid`
  (locals (cellExtent :type "Vector Structure") (currentY :type Integer) (currentX :type Integer) (currentCell :type "/Game/MazeGeneration/BP_Cell Object Reference"))
  (bind _currentcell (`local.currentCell`))
  (bind _currentcell_2 (`local.currentCell`))
  (`KismetArrayLibrary.Array_Clear` (`self.Cells`))
  (`|ExecutionSequence`
    (:`then_0`
      (bind _returnvalue (`|SpawnActorFromClass` (`self.Cell`) (`self.GetTransform`) "Undefined" "MultiplyWithRoot" null null))
      (set `local.cellExtent` (* (`.BoxExtent` (`self.GetActorBounds` _returnvalue false false)) 2.0))
      (`self.K2_DestroyActor` _returnvalue))
    (:`then_1`
      (for _index (range (`self.SizeY`))
        (set `local.currentY` _index)
        (for _index_2 (range (`self.SizeX`))
          (set `local.currentX` _index_2)
          (bind _returnvalue_2 (`|SpawnActorFromClass` (`self.Cell`) (`KismetMathLibrary.MakeTransform` (+ (.location (`self.GetTransform`)) (`KismetMathLibrary.MakeVector` (* (`local.currentX`) (.x (`local.cellExtent`))) (* (`local.currentY`) (.y (`local.cellExtent`))))) (.rotation (`self.GetTransform`)) (.scale (`self.GetTransform`))) "Undefined" "MultiplyWithRoot" null null))
          (`KismetArrayLibrary.Array_Add` (`self.Cells`) _returnvalue_2))))
    (:`then_2`
      (for _index_3 (range (`self.SizeY`))
        (set `local.currentY` _index_3)
        (for _index_4 (range (`self.SizeX`))
          (set `local.currentX` _index_4)
          (bind _asbp_cell (cast `/Game/MazeGeneration/BP_Cell` (`self.Get Cell` (`local.currentX`) (`local.currentY`))))
          (set `local.currentCell` _asbp_cell)
          (`|ExecutionSequence`
            (:`then_0`
              (if (> (`local.currentX`) 0)
                (bind _asbp_cell_2 (cast `/Game/MazeGeneration/BP_Cell` (`self.Get Cell` (- (`local.currentX`) 1) (`local.currentY`))))
                (`/Game/MazeGeneration/BP_Cell.Make Neighbor` _currentcell "NewEnumerator3" _asbp_cell_2)
                (`/Game/MazeGeneration/BP_Cell.Make Neighbor` _asbp_cell_2 "NewEnumerator1" _currentcell)))
            (:`then_1`
              (if (> (`local.currentY`) 0)
                (bind _asbp_cell_3 (cast `/Game/MazeGeneration/BP_Cell` (`self.Get Cell` (`local.currentX`) (- (`local.currentY`) 1))))
                (`/Game/MazeGeneration/BP_Cell.Make Neighbor` _asbp_cell_3 "NewEnumerator2" _currentcell_2)
                (`/Game/MazeGeneration/BP_Cell.Make Neighbor` _currentcell_2 "NewEnumerator0" _asbp_cell_3)))))))))

(fn `UserConstructionScript`)