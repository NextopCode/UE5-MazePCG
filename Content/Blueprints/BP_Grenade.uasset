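; BP_Grenade is a timed grenade actor that explodes after a fixed fuse starting at BeginPlay.
; When the delay ends, a sphere overlap around it finds WorldDynamic actors and calls BlowUp on those that cast to BP_Cell.
; It then fires its RadialForce impulse, spawns an explosion particle at its location and destroys itself.
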(event `self.ReceiveBeginPlay`
  (`KismetSystemLibrary.Delay` 3.0)
  (bind _outactors (`KismetSystemLibrary.SphereOverlapActors` (`self.K2_GetActorLocation`) 200.0 (`|MakeArray` "ObjectTypeQuery2" :!type "EObjectTypeQuery Enum")))
  (for _array_element _outactors
    (bind _asbp_cell (cast `/Game/MazeGeneration/BP_Cell` _array_element))
    (`/Game/MazeGeneration/BP_Cell.Blow Up` _asbp_cell))
  (`RadialForceComponent.FireImpulse` (`self.RadialForce`))
  (`GameplayStatics.SpawnEmitterAtLocation` "/Game/StarterContent/Particles/P_Explosion.P_Explosion" (`self.K2_GetActorLocation`))
  (`self.K2_DestroyActor`))

(fn `UserConstructionScript`)