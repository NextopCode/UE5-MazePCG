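; Inventory component that holds an array of items up to a Size limit and keeps the owner's HUD in sync.
; AddItem appends an item while space remains and returns whether it succeeded.
; RemoveItem removes by index, though its guard runs the removal only when the array length is less than that index, which looks inverted.
; Both functions call UpdateInventory on OwnerHUD after changing the array.
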(fn `Add Item`
  (params (Item :type "/Game/Blueprints/Item_Data Structure"))
  (returns (IsSucceed :type Boolean))
  (if (< (`KismetArrayLibrary.Array_Length` (`self.Inventory`)) (`self.Size`))
    (`KismetArrayLibrary.Array_Add` (`self.Inventory`) (`local.Item`))
    (`/Game/Widgets/WBP_HUD.Update Inventory` (`self.Owner HUD`))
    (return true)
    (else
      (return false))))

(fn `Remove Item`
  (params (Index :type Integer))
  (if (< (`KismetArrayLibrary.Array_Length` (`self.Inventory`)) Index)
    (`KismetArrayLibrary.Array_Remove` (`self.Inventory`) (`local.Index`))
    (`/Game/Widgets/WBP_HUD.Update Inventory` (`self.Owner HUD`))))